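; A world ladder that builds itself in the construction script from a spline's length and offers the player a Use-key (E) interaction prompt.
; Rung meshes are added at each height step, scaled by the clamped width and thickness settings, with extra side meshes on every sixth step.
; At the last step the left and right support meshes are moved to the ladder's width and raised by the handrail height.
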(fn ConstructionScript
  (bind _spline (Variables|Default|GetSpline))
  (bind _heightstep (Variables|BasicParam|GetHeightStep))
  (bind _returnvalue (Spline|GetSplineLength _spline))
  (bind _returnvalue_2 (Math|Float|Division(WholeandRemainder) _returnvalue _heightstep))
  (for _index (range 0 _returnvalue_2)
    (LocalVariables|SetLocalIndex _index)
    (if (not (== (LocalVariables|GetLocalIndex) 0))
      (if (>= (LocalVariables|GetLocalIndex) _returnvalue_2)
        (Transformation|SetRelativeLocation (Variables|Default|GetStaticMesh_LadderSupportLeft) (Math|Vector|MakeVector 0.0 (* (Variables|BasicParam|GetDefaultWidthLadder) (Math|Float|Clamp(Float) (/ (Variables|BasicParam|GetWidthLadder) 1e+03) 0.1 5.0)) (+ (Utilities|MGetLocationZ (LocalVariables|GetLocalIndex)) (Variables|BasicParam|GetHeightHandrails))) false false)
        (Transformation|SetRelativeLocation (Variables|Default|GetStaticMesh_LadderSupportRight) (Math|Vector|MakeVector 0.0 (* (* (Variables|BasicParam|GetDefaultWidthLadder) (Math|Float|Clamp(Float) (/ (Variables|BasicParam|GetWidthLadder) 1e+03) 0.1 5.0)) -1.0) (+ (Utilities|MGetLocationZ (LocalVariables|GetLocalIndex)) (Variables|BasicParam|GetHeightHandrails))) false false)
        (else
          (bind _returnvalue_3 (AddComponent|AddStaticMeshComponent false (Math|Transform|MakeTransform (Math|Vector|MakeVector 0.0 0.0 (Utilities|MGetLocationZ (LocalVariables|GetLocalIndex))) "0, 0, 0" "1,1,1")))
          (Transformation|SetWorldScale3D _returnvalue_3 (Math|Vector|MakeVector 1.0 (Math|Float|Clamp(Float) (/ (Variables|BasicParam|GetWidthLadder) 1e+03) 0.1 5.0) (Math|Float|Clamp(Float) (/ (Variables|BasicParam|GetThicknessLadder) 1e+03) 0.1 5.0)))
          (if (== (Math|Integer|%(Integer) (LocalVariables|GetLocalIndex) 6) 0)
            (AddComponent|AddStaticMeshComponent false (Math|Transform|MakeTransform (Math|Vector|MakeVector 0.0 (* (Variables|BasicParam|GetDefaultWidthLadder) (Math|Float|Clamp(Float) (/ (Variables|BasicParam|GetWidthLadder) 1e+03) 0.1 5.0)) (Utilities|MGetLocationZ (LocalVariables|GetLocalIndex))) "0, 0, 0" "1,1,1"))
            (AddComponent|AddStaticMeshComponent false (Math|Transform|MakeTransform (Math|Vector|MakeVector 0.0 (* (* (Variables|BasicParam|GetDefaultWidthLadder) (Math|Float|Clamp(Float) (/ (Variables|BasicParam|GetWidthLadder) 1e+03) 0.1 5.0)) -1.0) (Utilities|MGetLocationZ (LocalVariables|GetLocalIndex))) "0, 0, 0" "1,1,1"))))))))

(fn InterfaceInteractionwithPlayer
  (return true true true (Variables|BasicParam|GetTextInteraction)))