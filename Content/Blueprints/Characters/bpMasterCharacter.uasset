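; Master player character with walk/run, jump and flip, crouch, prone, sword attacks and weapon equip animations.
; A camera sphere trace each Tick queries hit actors through an interaction interface and shows their prompt in WInteraction.
; The MStopMove macro gates most actions on MoveEnabled, which Prone clears during transition montages.
; Stance changes adjust capsule, speed or mesh offset; holding right mouse switches rotation to follow the controller.
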(event EventTick
  (params (DeltaSeconds :type Float%20%28single-precision%29))
  (bind _camera (Variables|Default|GetCamera))
  (bind _returnvalue (Transformation|GetWorldLocation _camera))
  (bind (_outhit _returnvalue_2) (Collision|SphereTraceByChannel _returnvalue (+ _returnvalue (* (Math|Vector|GetForwardVector _camera) 5e+02)) 1e+01 "TraceTypeQuery1" false 0 "None" true "(R=1.000000,G=0.000000,B=0.000000,A=1.000000)" "(R=0.000000,G=1.000000,B=0.000000,A=1.000000)" 0.0))
  (if _returnvalue_2
    (if (not (Variables|Default|GetisInteraction?))
      (bind (_succesfull_ _usekeye_ _isshowmessageaddional_ _text) (Class|BpInteraceItemWorld|InterfaceInteractionwithPlayer(Message) (.HitActor (Collision|BreakHitResult _outhit))))
      (if _succesfull_
        (Variables|Default|SetActorInteraction (.HitActor (Collision|BreakHitResult _outhit)))
        (Rendering|Debug|DrawDebugSphere (.Location (Collision|BreakHitResult _outhit)) 1e+01 12 "(R=0.147312,G=1.000000,B=0.000000,A=1.000000)" 0.0)
        (Default|FShowMessage (Variables|Default|GetwInteraction) _usekeye_ _isshowmessageaddional_ _text)))
    (elif (not (Variables|Default|GetisInteraction?))
      (Variables|Default|GetActorInteraction
        (:then
          (Variables|Default|SetActorInteraction 0)
          (Variables|Default|SetisInteraction? false)
          (Default|FShowMessage (Variables|Default|GetwInteraction) false false))
        (:else)))))

(event EventBeginPlay
  (Utilities|FlowControl|Sequence
    (:then_0
      (bind _returnvalue (UserInterface|CreateWidget "/Game/Blueprints/widgets/wInfoInteraction.wInfoInteraction_C"))
      (bind _output_get (Variables|Default|SetwInteraction _returnvalue))
      (UserInterface|Viewport|AddtoViewport _output_get 0)
      (Default|FShowMessage (Variables|Default|GetwInteraction) false false))))

(event Custom|equipWeapon
  ;[1 0.1834 0.5005] B
  (Utilities|MStopMove
    (:MoveOn
      (Variables|Default|SetisEquip? true)
      (bind _returnvalue (Animation|Montage|MontagePlay (Components|SkeletalMesh|GetAnimInstance (Variables|Character|GetMesh)) (select (Variables|Default|GetisEquipWeaponSword?) (Variables|AnimMontages|GetStanding_Disarm_Over_Shoulder_Montage) (Variables|AnimMontages|GetUnarmed_Equip_Over_Shoulder_Montage)) 1.0 "MontageLength" 0.0 true))
      (Utilities|FlowControl|Delay _returnvalue)
      (Variables|Default|SetisEquip? false)
      (Variables|Default|SetmoveEnabled? true)
      (if (Variables|Default|GetisProne?)
        ;[1 1 1] P key - Prone
        (|Prone
          (:false
            ;[1 1 1] LeftCtrl
            (Character|Crouch)))))))

(event Input|ActionEvents|InputActionJump
  (params (Key :type Key%20Structure))
  ;[1 0.1834 0.5005] Comment
  (:Pressed
    (Utilities|MStopMove
      (:MoveOn
        (if (not (Variables|Default|GetisProne?))
          (if (Variables|Default|GetisRightMouseBtn?)
            (Animation|Montage|MontagePlay (Components|SkeletalMesh|GetAnimInstance (Variables|Character|GetMesh)) (Variables|AnimMontages|GetRunning_Forward_Flip_Montage) 1.0 "MontageLength" 0.0 true)
            (else
              (Character|Jump)))))))
  (:Released
    (Character|StopJumping)))

(event Input|AxisEvents|InputAxisMoveForward
  (params (AxisValue :type Float%20%28single-precision%29))
  ;[1 0.1834 0.5005] Comment
  (Utilities|MStopMove
    (:MoveOn
      (Pawn|Input|AddMovementInput (Math|Vector|GetForwardVector (Math|Rotator|MakeRotator 0.0 0.0 (.Yaw (Math|Rotator|BreakRotator (Pawn|GetControlRotation :!class /Script/Engine.Pawn))))) AxisValue false))))

(event Input|AxisEvents|InputAxisMoveRight
  (params (AxisValue :type Float%20%28single-precision%29))
  ;[1 0.1834 0.5005] Comment
  (Utilities|MStopMove
    (:MoveOn
      (Pawn|Input|AddMovementInput (Math|Vector|GetRightVector (Math|Rotator|MakeRotator 0.0 0.0 (.Yaw (Math|Rotator|BreakRotator (Pawn|GetControlRotation :!class /Script/Engine.Pawn))))) AxisValue false))))

(event Input|AxisEvents|InputAxisLookUp
  (params (AxisValue :type Float%20%28single-precision%29))
  ;[1 0.1834 0.5005] Comment
  (Pawn|Input|AddControllerPitchInput AxisValue))

(event Input|AxisEvents|InputAxisTurnRate
  (params (AxisValue :type Float%20%28single-precision%29))
  ;[1 0.1834 0.5005] Comment
  (Pawn|Input|AddControllerYawInput AxisValue))

(event Input|KeyboardEvents|B
  (params (Key :type Key%20Structure))
  ;[1 0.1834 0.5005] B
  (:Pressed
    (Utilities|MStopMove
      (:MoveOn
        (Variables|Default|SetisEquip? true)
        (bind _returnvalue (Animation|Montage|MontagePlay (Components|SkeletalMesh|GetAnimInstance (Variables|Character|GetMesh)) (select (Variables|Default|GetisEquipWeaponSword?) (Variables|AnimMontages|GetStanding_Disarm_Over_Shoulder_Montage) (Variables|AnimMontages|GetUnarmed_Equip_Over_Shoulder_Montage)) 1.0 "MontageLength" 0.0 true))
        (Utilities|FlowControl|Delay _returnvalue)
        (Variables|Default|SetisEquip? false)
        (Variables|Default|SetmoveEnabled? true)
        (if (Variables|Default|GetisProne?)
          ;[1 1 1] P key - Prone
          (|Prone
            (:false
              ;[1 1 1] LeftCtrl
              (Character|Crouch))))))))

(event Input|KeyboardEvents|C
  (params (Key :type Key%20Structure))
  (:Pressed
    (Animation|Montage|MontagePlay (Components|SkeletalMesh|GetAnimInstance (Variables|Character|GetMesh)) "/Game/mixamoCharacters/Aj_RB/AnimRB/AnimRB/Sprint_To_Wall_Climb_Montage.Sprint_To_Wall_Climb_Montage" 1.0 "MontageLength" 0.0 true)))

(event Input|MouseEvents|LeftMouseButton
  (params (Key :type Key%20Structure))
  ;[1 1 1] LeftMouseButton - Attack
  (:Pressed
    (Utilities|MStopMove
      (:MoveOn
        (Utilities|FlowControl|Sequence
          (:then_0
            (if (not (Variables|Default|GetisEquip?))
              (if (Variables|Default|GetisEquipWeaponSword?)
                (if (not (AI|Components|NavMovement|IsFalling (Variables|Character|GetCharacterMovement)))
                  (switch int (Variables|Default|GetidAttack)
                    (:0
                      (Animation|Montage|MontagePlay (Components|SkeletalMesh|GetAnimInstance (Variables|Character|GetMesh)) (Variables|AnimMontages|GetStanding_Melee_Attack_Horizontal_Montage) 1.0 "MontageLength" 0.0 true)
                      (Variables|Default|SetidAttack 1))
                    (:1
                      (Animation|Montage|MontagePlay (Components|SkeletalMesh|GetAnimInstance (Variables|Character|GetMesh)) (Variables|AnimMontages|GetStanding_Melee_Run_Jump_Attack_Montage) 1.0 "MontageLength" 0.0 true)
                      (Variables|Default|SetidAttack 0)))))))
          (:then_1
            (if (Variables|Default|GetisProne?)
              (Animation|Montage|MontagePlay (Components|SkeletalMesh|GetAnimInstance (Variables|Character|GetMesh)) (Variables|AnimMontages|GetThrow_Grenade1_Montage) 1.0 "MontageLength" 0.0 true))))))))

(event Input|KeyboardEvents|CapsLock
  (params (Key :type Key%20Structure))
  (bind _charactermovement (Variables|Character|GetCharacterMovement))
  ;[1 1 1] CapsLock - Ходьба / Бег
  (:Pressed
    (bind _output_get (Variables|Default|SetisRunning? (not (Variables|Default|GetisRunning?))))
    (if _output_get
      (Variables|/Script/Engine.CharacterMovementComponent|SetMaxWalkSpeed _charactermovement 6e+02)
      (else
        (Variables|/Script/Engine.CharacterMovementComponent|SetMaxWalkSpeed _charactermovement 2e+02)))))

(event Input|KeyboardEvents|LeftCtrl
  (params (Key :type Key%20Structure))
  ;[1 1 1] LeftCtrl
  (:Pressed
    (if (not (AI|Components|NavMovement|IsFalling (Variables|Character|GetCharacterMovement)))
      (Utilities|MStopMove
        (:MoveOn
          (if (not (Variables|Default|GetisProne?))
            (Variables|Default|SetisCrouching? (not (Variables|Default|GetisCrouching?)))
            (Character|Crouch :!label _label)
            (else
              ;[1 1 1] P key - Prone
              (Variables|Default|SetisCrouching? true)
              (Variables|Default|SetisProne? (not (Variables|Default|GetisProne?)))
              (if (not (Variables|Default|GetisEquipWeaponSword?))
                (|Prone
                  (:false
                    (goto _label)))
                (else
                  (CallFunction|EquipWeapon))))))))))

(event Input|KeyboardEvents|P
  (params (Key :type Key%20Structure))
  ;[1 1 1] P key - Prone
  (:Pressed
    (if (not (AI|Components|NavMovement|IsFalling (Variables|Character|GetCharacterMovement)))
      (Utilities|MStopMove
        (:MoveOn
          (if (Variables|Default|GetisProne?)
            (Variables|Default|SetisCrouching? false))
          (Variables|Default|SetisProne? (not (Variables|Default|GetisProne?)))
          (if (not (Variables|Default|GetisEquipWeaponSword?))
            (|Prone
              (:false
                ;[1 1 1] LeftCtrl
                (Character|Crouch)))
            (else
              (CallFunction|EquipWeapon))))))))

(event Input|MouseEvents|RightMouseButton
  (params (Key :type Key%20Structure))
  (bind _charactermovement (Variables|Character|GetCharacterMovement))
  (bind _charactermovement_2 (Variables|Character|GetCharacterMovement))
  ;[1 1 1] RightMouseButton
  (:Pressed
    (Variables|Default|SetisRightMouseBtn? true)
    (Variables|/Script/Engine.CharacterMovementComponent|SetbUseControllerDesiredRotation _charactermovement_2 true)
    (Variables|/Script/Engine.CharacterMovementComponent|SetbOrientRotationToMovement _charactermovement_2 false))
  (:Released
    (Variables|Default|SetisRightMouseBtn? false)
    (Variables|/Script/Engine.CharacterMovementComponent|SetbUseControllerDesiredRotation _charactermovement false)
    (Variables|/Script/Engine.CharacterMovementComponent|SetbOrientRotationToMovement _charactermovement true)))

(fn ConstructionScript
  (Variables|/Script/Engine.SkinnedMeshComponent|GetSkeletalMesh (Variables|Character|GetMesh)
    (:then
      (Transformation|AttachComponentToComponent (Variables|Default|GetNeckSocket) (Variables|Character|GetMesh) "NeckSocket" "KeepRelative" "KeepRelative" "KeepRelative" true)
      (Transformation|AttachComponentToComponent (Variables|Default|GetRightHandSocket) (Variables|Character|GetMesh) "RightHandSocket" "KeepRelative" "KeepRelative" "KeepRelative" true)
      (Transformation|SetRelativeTransform (Variables|Default|GetWeapon) (Math|Transform|MakeTransform "0, 0, 0" "0, 0, 0" "1,1,1") false false))
    (:else)))